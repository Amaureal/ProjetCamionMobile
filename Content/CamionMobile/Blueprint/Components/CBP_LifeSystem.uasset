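; Life component that tracks an owner's current life, maximum life and dead state.
; Heal and Damage route through SetLife, which floors and clamps the value, then broadcasts OnLifeUpdate with the value and its 0-1 percentage.
; When the percentage reaches zero, SetLife flags IsDead and fires OnDie.
; ResetLife restores full life, clears the dead flag and optionally rebroadcasts the update through SetLife.
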(event `self.ReceiveBeginPlay`)

(fn `Damage`
  (params (Amount :type "Float (double-precision)"))
  (`self.Set Life` (- (`self.CurLife`) Amount)))

(fn `Heal`
  (params (Amount :type "Float (double-precision)"))
  (`self.Set Life` (+ (`self.CurLife`) Amount)))

(fn `Reset Life`
  (params (`Update Life` :type Boolean))
  (set `self.CurLife` (`self.MaxLife`))
  (set `self.IsDead` false)
  (if `Update Life`
    (`self.Set Life` (`self.CurLife`))))

(fn `Set Life`
  (params (`New Life` :type "Float (double-precision)"))
  (bind _maxlife (`self.MaxLife`))
  ;[1 1 1] Updates the life value and transforms it into a percentage (between 0 and 1), sends the life update to the object. If the life value is equal to 0, sends: On Die.
  (bind _output_get (set `self.CurLife` (`KismetMathLibrary.FClamp` (`KismetMathLibrary.Conv_IntToDouble` (`KismetMathLibrary.FFloor` `New Life`)) 0.0 _maxlife)))
  (bind _output_get_2 (set `self.Percent` (`KismetMathLibrary.SafeDivide` _output_get _maxlife)))
  (`self.OnLifeUpdate` (`self.CurLife`) _output_get_2)
  (if (== _output_get_2 0.0)
    (set `self.IsDead` true)
    (`self.OnDie`)))