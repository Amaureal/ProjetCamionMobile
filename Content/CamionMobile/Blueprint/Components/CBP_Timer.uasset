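; CBP_Timer is a countdown timer component that broadcasts its remaining minutes and seconds and signals when time runs out.
; ResetTimer refills the time and announces a start, but does not itself begin the countdown.
; Decompt re-calls itself after a speed-scaled Delay, removing one second per pass until TimeOut fires at zero.
; ModifieTimer clamps and floors the time, splitting it for the NewTime dispatcher.
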(event `Reset Timer`
  (`self.Timer as started`)
  (bind _output_get (set `self.CurSeconds` (`self.MaxSecondes`)))
  (`self.Modifie Timer` _output_get)
  (set `self.Time Out` false))

(event `Decompt`
  (params (Time :type "Float (double-precision)"))
  (bind _output_get (set `self.CurSeconds` (`KismetMathLibrary.FClamp` (- Time 1.0) 0.0 (`self.MaxSecondes`))))
  (`self.Modifie Timer` _output_get)
  (if (> (`self.CurSeconds`) 0.0)
    (`KismetSystemLibrary.Delay` (/ 1.0 (`self.Time Speed`)))
    (`self.Decompt` (`self.CurSeconds`))
    (else
      (`self.TimeOut`))))

(event `Modifie Timer`
  (params (`New Time` :type "Float (double-precision)"))
  (bind _list_time (`self.List Time`))
  (bind _output (`|GetArrayItem` _list_time 1))
  (bind _returnvalue (`KismetMathLibrary.FFloor` (`KismetMathLibrary.FClamp` `New Time` 0.0 (`self.MaxSecondes`))))
  (bind _output_get (set `self.CurSeconds` (`KismetMathLibrary.Conv_IntToDouble` _returnvalue)))
  (`KismetArrayLibrary.Array_Set` _list_time 1 (`KismetMathLibrary.FFloor` (/ _output_get 60.0)))
  (`KismetArrayLibrary.Array_Set` _list_time 0 (- _returnvalue (* _output 60)))
  (`self.New Time` (`|GetArrayItem` _list_time) _output))

(event `TimeOut`
  (set `self.Time Out` true)
  (`self.Modifie Timer` (`self.CurSeconds`))
  (`self.Timer Out`))